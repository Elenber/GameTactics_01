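; Player controller for a team-based building game, linking team and color selection, gameplay UI, grid building and chat.
; Team choice updates the game state, player state and camera pawn.
; Left-click traces under the cursor to highlight and store a same-team grid cell; building spends player-state coins and spawns through the camera pawn.
; Chat messages fan out through every player state, and UpdateChat appends to the gameplay widget.
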(event Custom|SendMessageToServer
  (params (Message :type Text))
  ;[1 1 1] ChatSystem
  (Variables|Chat|SetSenderText Message)
  (Variables|Chat|SetSenderName (Utilities|Text|ToText(String) (Variables|/Script/Engine.PlayerState|GetPlayerName (.AsMy%20Player%20State (Utilities|Casting|CastToMyPlayerState (Variables|GetPlayerState))))))
  (bind _asmy_game_state (Utilities|Casting|CastToMyGameState (Game|GetGameState)))
  (for _array_element (Variables|/Script/Engine.GameStateBase|GetPlayerArray _asmy_game_state)
    (bind _asmy_player_state (Utilities|Casting|CastToMyPlayerState _array_element))
    (Default|MessagetoController _asmy_player_state (Variables|Chat|GetSenderName) (Variables|Chat|GetSenderText))))

(event Custom|SetGameMode
  (params (GameMode :type Integer))
  ;[1 1 1] SetUpPlayerForNewGameMode
  (Variables|Default|SetGameMode GameMode))

(event Custom|UpdateChat
  (params (Message :type Text) (Sender :type Text))
  (bind _gameplaywb (Variables|Default|GetGamePlayWB))
  (bind _newchatwindow (Variables|/Game/UI/GameplayUI/GameplayWB.GameplayWB_C|GetNewChatWindow _gameplaywb))
  ;[1 1 1] ChatSystem
  (Utilities|IsValid _newchatwindow
    (:Is%20Valid
      (Default|AddChildtoChat _newchatwindow Message Sender))))

(event Custom|AddGamePlayWB
  ;[1 1 1] ControllerIncludedInTheTeamWithColor
  (bind _returnvalue (UserInterface|CreateWidget "/Game/UI/GameplayUI/GameplayWB.GameplayWB_C"))
  (bind _output_get (Variables|Default|SetGamePlayWB _returnvalue))
  (UserInterface|Viewport|AddtoViewport _output_get 0)
  (Input|SetInputModeGameandUI self (Variables|Default|GetGamePlayWB) "DoNotLock" false))

(event Custom|BuildTowerOrBarracs
  (params (NumberOfBuilds :type Integer))
  (bind _playerstate (Variables|GetPlayerState))
  (bind _asmy_player_state (Utilities|Casting|CastToMyPlayerState _playerstate))
  ;[1 1 1] Building
  (if (>= (Variables|/Game/Blueprints/Gameplay/MyPlayerState.MyPlayerState_C|GetCoins _asmy_player_state) 5)
    (Variables|/Game/Blueprints/Gameplay/MyPlayerState.MyPlayerState_C|SetCoins _asmy_player_state (- (Variables|/Game/Blueprints/Gameplay/MyPlayerState.MyPlayerState_C|GetCoins _asmy_player_state) 5))
    (Variables|Building|SetNumberOfBuilds NumberOfBuilds)
    (bind _aspawn_camera (Utilities|Casting|CastToPawnCamera (Pawn|GetControlledPawn)))
    (Variables|Building|SetCanBuild false)
    (Default|SpawnBuilds _aspawn_camera (Variables|Building|GetLocationBuild) (Variables|Building|GetNumberOfBuilds))))

(event Custom|SetColorEnumAndTeam
  (params (Team :type Integer) (ColorEnum :type Integer) (MaterialIsntance :type Material%20Instance%20Object%20Reference))
  ;[1 1 1] ControllerIncludedInTheTeamWithColor
  (Variables|TeamLogic|SetTeam Team)
  (Variables|TeamLogic|SetColorEnum ColorEnum)
  (Variables|Building|SetMaterialIsntance MaterialIsntance)
  (bind _asmy_game_state (Utilities|Casting|CastToMyGameState (Game|GetGameState)))
  (Default|SwitchOffColorEnum _asmy_game_state (Variables|TeamLogic|GetColorEnum))
  (bind _asmy_player_state (Utilities|Casting|CastToMyPlayerState (Variables|GetPlayerState)))
  (Variables|/Game/Blueprints/Gameplay/MyPlayerState.MyPlayerState_C|SetColorEnum _asmy_player_state (Variables|TeamLogic|GetColorEnum))
  (bind _aspawn_camera (Utilities|Casting|CastToPawnCamera (Pawn|GetControlledPawn)))
  (Default|GetfromPCVar _aspawn_camera (Variables|Building|GetMaterialIsntance) (Variables|TeamLogic|GetTeam)))

(event Custom|UpdateAllVariables
  (params (SelectedGrid :type Grid%20Base%20Object%20Reference) (NumberOfBuilds :type Integer) (LocationBuild :type Vector) (Team :type Integer) (ColorEnum :type Integer))
  ;[1 1 1] Building
  (Variables|Building|SetCanBuild true)
  (Variables|Building|SetSelectedGrid SelectedGrid)
  (Variables|Building|SetNumberOfBuilds NumberOfBuilds)
  (Variables|Building|SetLocationBuild LocationBuild)
  (Variables|TeamLogic|SetTeam Team)
  (Variables|TeamLogic|SetColorEnum ColorEnum))

(event Custom|HideLoadingScreen
  ;[1 1 1] SetUpPlayerForNewGameMode
  (bind _asmy_game_instance (Utilities|Casting|CastToMyGameInstance (Game|GetGameInstance)))
  (Default|HideLoadingScreen _asmy_game_instance))

(event Custom|CreateGameUI
  ;[1 1 1] SetUpPlayerForNewGameMode
  (bind _returnvalue (UserInterface|CreateWidget "/Game/UI/GameplayUI/TeamAndColorSelectWB.TeamAndColorSelectWB_C"))
  (bind _output_get (Variables|Default|SetSelectTeamWB _returnvalue))
  (UserInterface|Viewport|AddtoViewport _output_get 0)
  (Input|SetInputModeUIOnly self (Variables|Default|GetSelectTeamWB) "DoNotLock"))

(event EventBeginPlay
  ;[1 1 1] SetUpPlayerForNewGameMode
  (Variables|Default|SetbShowMouseCursor true))

(event Input|MouseEvents|LeftMouseButton
  (params (Key :type Key%20Structure))
  (bind _returnvalue (Game|GetPlayerController 0))
  (bind (_worldlocation _worlddirection) (Game|Player|ConvertMouseLocationToWorldSpace _returnvalue))
  ;[1 1 1] Building
  (:Pressed
    (bind (_outhit _returnvalue_2) (Collision|LineTraceForObjects _worldlocation (+ _worldlocation (* _worlddirection 2e+03)) (Utilities|Array|MakeArray "ObjectTypeQuery7") false (Utilities|Array|MakeArray self) "None"))
    (if _returnvalue_2
      (bind _outactors (Actor|GetAllActorsOfClass "/Game/Blueprints/Gameplay/Grid/MyGridBase.MyGridBase_C"))
      (for _array_element _outactors
        (Rendering|SetVisibility (Variables|/Game/Blueprints/Gameplay/Grid/MyGridBase.MyGridBase_C|GetPlane _array_element) false false))
      (bind _asmy_grid_base (Utilities|Casting|CastToMyGridBase (.HitActor (Collision|BreakHitResult _outhit))))
      (if (== (Variables|TeamLogic|GetTeam) (Variables|/Game/Blueprints/Gameplay/Grid/MyGridBase.MyGridBase_C|GetTeam _asmy_grid_base))
        (Variables|Building|SetLocationBuild (Variables|/Game/Blueprints/Gameplay/Grid/MyGridBase.MyGridBase_C|GetLocationGrid _asmy_grid_base))
        (CallFunction|UpdateAllVariables (Variables|Building|GetSelectedGrid) (Variables|Building|GetNumberOfBuilds) (Variables|Building|GetLocationBuild) (Variables|TeamLogic|GetTeam) (Variables|TeamLogic|GetColorEnum))
        (Rendering|SetVisibility (Variables|/Game/Blueprints/Gameplay/Grid/MyGridBase.MyGridBase_C|GetPlane _asmy_grid_base) true false)))))

(event Input|KeyboardEvents|Tab
  (params (Key :type Key%20Structure))
  ;[1 1 1] ChatSystem
  (:Pressed
    (Viewport|RemoveAllWidgets)
    (bind _returnvalue (UserInterface|CreateWidget "/Game/UI/GameplayUI/TeamAndColorSelectWB.TeamAndColorSelectWB_C"))
    (bind _output_get (Variables|Default|SetSelectTeamWB _returnvalue))
    (UserInterface|Viewport|AddtoViewport _output_get 0)
    (Input|SetInputModeUIOnly self (Variables|Default|GetSelectTeamWB) "DoNotLock")))

(fn ConstructionScript)